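; BP_PROP_treasurechest4 is an interactable treasure chest that opens and spawns a crystal pickup.
; Collision overlap toggles a text prompt, which interaction hides while a timeline rotates the lid.
; A DoOnce on the timeline update spawns BP_PickUp_Crystal at the chest after a short delay.
; Both widget overlap events hide the widget through an Open-check macro, and nothing here sets Open.
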(event OnComponentBeginOverlap(Collision)
  (params (OverlappedComponent :type Primitive%20Component%20Object%20Reference) (OtherActor :type Actor%20Object%20Reference) (OtherComp :type Primitive%20Component%20Object%20Reference) (OtherBodyIndex :type Integer) (bFromSweep :type Boolean) (SweepResult :type Hit%20Result%20Structure%20%28by%20ref%29))
  ;[1 1 1] Text
  (Rendering|SetVisibility (Variables|Default|GetTextRender) true false))

(event OnComponentEndOverlap(Collision)
  (params (OverlappedComponent :type Primitive%20Component%20Object%20Reference) (OtherActor :type Actor%20Object%20Reference) (OtherComp :type Primitive%20Component%20Object%20Reference) (OtherBodyIndex :type Integer))
  ;[1 1 1] Text
  (Rendering|SetVisibility (Variables|Default|GetTextRender) false false))

(event EventBeginPlay
  ;[1 1 1] Text
  (Rendering|SetVisibility (Variables|Default|GetTextRender) false false))

(event EventOnBeginOverlab
  ;[1 1 1] ChestWidget
  (Utilities|OpenMac
    (:true
      (Rendering|SetVisibility (Variables|Default|GetWidget) false false))))

(event EventOnEndOverlab
  ;[1 1 1] ChestWidget
  (Utilities|OpenMac
    (:true
      (Rendering|SetVisibility (Variables|Default|GetWidget) false false))))

(event EventOnInteractBegin
  ;[1 1 1] ChestInteract
  ;;[1 1 1] Text
  (Rendering|SetVisibility (Variables|Default|GetTextRender) false false)
  ;;[1 1 1] ChestAnimation
  (bind _newtrack_0 (Timeline|Play Play)
    (:Update
      (Transformation|SetRelativeRotation (Variables|Default|GetSM_PROP_treasurechest_top) (Math|Rotator|MakeRotator _newtrack_0 0.0 0.0) false false)
      ;;[1 1 1] ChestSpawn
      (Utilities|FlowControl|DoOnce false
        (:Completed
          (Utilities|FlowControl|Delay 0.7)
          (Game|SpawnActorfromClass "/Game/SlimeLab/PickUpAndCrystal/BP_PickUp_Crystal.BP_PickUp_Crystal_C" (Math|Transform|MakeTransform (Transformation|GetActorLocation) (Transformation|GetActorRotation) (+ (Transformation|GetActorScale3D) 1.0)) "AdjustIfPossibleButAlwaysSpawn" (Variables|Default|GetCrystal) (Variables|Default|GetMainCharacter)))))))

(event EventOnInteractEnd
  ;[1 1 1] ChestInteract
)

(fn ConstructionScript)