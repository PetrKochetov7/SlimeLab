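; StatusCharacter tracks a character's HP and signals when it runs out.
; CurrentHP starts at MaxHP on BeginPlay.
; MakeDamageHealth subtracts the given value and clamps the result between zero and MaxHP, so negative values heal.
; It calls the OnDeath dispatcher whenever the result is zero, with no guard against repeat calls; Tick is empty.
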(event EventBeginPlay
  ;[1 1 1] HP Status
  (Variables|Default|SetCurrentHP (Variables|Default|GetMaxHP)))

(event EventTick
  (params (DeltaSeconds :type Float%20%28single-precision%29))
  ;[1 1 1] HP Status
)

(fn MakeDamage/Health
  (params (Value :type Float%20%28single-precision%29))
  (Variables|Default|SetCurrentHP (Math|Float|Clamp(Float) (- (Variables|Default|GetCurrentHP) Value) 0.0 (Variables|Default|GetMaxHP)))
  (if (<= (Variables|Default|GetCurrentHP) 0.0)
    (Default|CallOnDeath)))