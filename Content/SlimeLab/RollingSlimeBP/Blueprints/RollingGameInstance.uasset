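; Game instance for the rolling slime game that persists the best crystal count for each level.
; On Init it loads the save object from a single fixed slot, or creates a new one if no save is found.
; AddCrystals records a level's count only when the level is new or the count beats the stored value, then immediately writes the save to disk.
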(event EventInit
  (CallFunction|LoadfromHdd))

(fn SavetoHdd
  (SaveGame|SaveGametoSlot (Variables|Default|GetCurrentSaveObject) "1"))

(fn LoadfromHdd
  (bind _returnvalue (SaveGame|LoadGamefromSlot "1"))
  (if (Utilities|IsValid _returnvalue)
    (bind _assave_game_object (Utilities|Casting|CastToSaveGameObject _returnvalue))
    (Variables|Default|SetCurrentSaveObject _assave_game_object)
    (else
      (bind _returnvalue_2 (SaveGame|CreateSaveGameObject "/Game/SlimeLab/SaveSystem/SaveGameObject.SaveGameObject_C"))
      (Variables|Default|SetCurrentSaveObject _returnvalue_2))))

(fn AddCrystals
  (params (Level :type String) (NumOfCry :type Integer))
  (bind _currentsaveobject (Variables|Default|GetCurrentSaveObject))
  (bind _leveldata (Variables|/Game/SlimeLab/SaveSystem/SaveGameObject.SaveGameObject_C|GetLevelData _currentsaveobject))
  (bind (_value _returnvalue) (Utilities|Map|Find _leveldata Level))
  (if _returnvalue
    (if (> NumOfCry (.NumbOfCrystal (Utilities|Struct|BreakLevelDataStruct _value)))
      (Default|AddData (Variables|Default|GetCurrentSaveObject) Level NumOfCry)
      (CallFunction|SavetoHdd :!label _label))
    (else
      (Default|AddData (Variables|Default|GetCurrentSaveObject) Level NumOfCry)
      (goto _label))))