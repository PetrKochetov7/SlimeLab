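; VictoryExitGateBase is an exit gate that shows the victory screen when something overlaps its box.
; The first box overlap, gated by DoOnce with no actor filter, reveals a TextRender and adds a VictoryWidget to the viewport, creating it if needed.
; The text hides on BeginPlay and end overlap, so later overlaps never reshow it.
; Activate, CheckCondition and construction only call the parent class.
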(event OnComponentBeginOverlap(Box)
  (params (OverlappedComponent :type Primitive%20Component%20Object%20Reference) (OtherActor :type Actor%20Object%20Reference) (OtherComp :type Primitive%20Component%20Object%20Reference) (OtherBodyIndex :type Integer) (bFromSweep :type Boolean) (SweepResult :type Hit%20Result%20Structure%20%28by%20ref%29))
  ;[1 1 1] VictoryInteract
  (Utilities|FlowControl|DoOnce false
    (:Completed
      (Rendering|SetVisibility (Variables|Default|GetTextRender) true false)
      (Variables|Default|GetVictoryWidget
        (:then
          _)
        (:else
          (bind _returnvalue (UserInterface|CreateWidget "/Game/SlimeLab/VictoryAndStartExit/VictoryWidgetBlueprint.VictoryWidgetBlueprint_C"))
          (Variables|Default|SetVictoryWidget _returnvalue)))
      (UserInterface|Viewport|AddtoViewport (Variables|Default|GetVictoryWidget) 0))))

(event OnComponentEndOverlap(Box)
  (params (OverlappedComponent :type Primitive%20Component%20Object%20Reference) (OtherActor :type Actor%20Object%20Reference) (OtherComp :type Primitive%20Component%20Object%20Reference) (OtherBodyIndex :type Integer))
  ;[1 1 1] Text
  (Rendering|SetVisibility (Variables|Default|GetTextRender) false false))

(event EventBeginPlay
  ;[1 1 1] Text
  (|CallParentFunction)
  (Rendering|SetVisibility (Variables|Default|GetTextRender) false false))

(event Collision|EventActorBeginOverlap
  (params (OtherActor :type Actor%20Object%20Reference))
  (|CallParentFunction OtherActor))

(event EventTick
  (params (DeltaSeconds :type Float%20%28single-precision%29))
  (|CallParentFunction DeltaSeconds))

(fn ConstructionScript
  (|CallParentFunction))

(fn Activate
  (|CallParentFunction))

(fn CheckCondition
  (return (|CallParentFunction)))