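; Lever actor that opens the StoneInPass1 stone whose DoorValue matches its LeverValue.
; Activate plays a one-time sound and timeline rotation of the lever, then hides its text and calls StoneDown on the first matching stone.
; The camera blends to that stone and returns to the player pawn after a delay.
; CheckCondition always passes, and only the lever animation is guarded by DoOnce.
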(event Custom|OpenStone
  (params (Player :type Main%20Character%20Object%20Reference))
  (Rendering|SetVisibility (Variables|Default|GetTextRender) false false)
  (bind _outactors (Actor|GetAllActorsOfClass "/Game/SlimeLab/LeversAndStonePass/StoneInPass1.StoneInPass1_C"))
  (bind _array_element (Utilities|Array|ForEachLoopwithBreak _outactors :!label _label)
    (:LoopBody
      (if (== (Variables|/Game/SlimeLab/LeversAndStonePass/StoneInPass1.StoneInPass1_C|GetDoorValue _array_element) (Variables|Default|GetLeverValue))
        (Default|StoneDown _array_element Player)
        (Game|Player|SetViewTargetwithBlend (Game|GetPlayerController 0) _array_element 2.0 "VTBlend_Linear" 0.0 false)
        (Utilities|FlowControl|Delay 4.0)
        (Game|Player|SetViewTargetwithBlend (Game|GetPlayerController 0) (Game|Player|GetPlayerPawn 0) 2.0 "VTBlend_Linear" 0.0 false)
        (goto _label Break)))))

(event Custom|LeverActivate
  (Utilities|FlowControl|DoOnce false
    (:Completed
      (Audio|PlaySoundatLocation "/Game/SlimeLab/LeversAndStonePass/SoundStoneOpen2Sec.SoundStoneOpen2Sec" (Transformation|GetActorLocation) "0, 0, 0" 1.0 1.0 0.0 0 0 0)
      (bind _newtrack_0 (Timeline|Timeline_0 Play)
        (:Update
          (Transformation|SetRelativeRotation (Variables|Default|GetCube1) (Math|Rotator|MakeRotator _newtrack_0 0.0 0.0) false false))))))

(event EventBeginPlay
  (|CallParentFunction) ; This node is disabled and will not be called.\nDrag off pins to build functionality.
)

(event Collision|EventActorBeginOverlap
  (params (OtherActor :type Actor%20Object%20Reference))
  (|CallParentFunction OtherActor) ; This node is disabled and will not be called.\nDrag off pins to build functionality.
)

(event EventTick
  (params (DeltaSeconds :type Float%20%28single-precision%29))
  (|CallParentFunction DeltaSeconds) ; This node is disabled and will not be called.\nDrag off pins to build functionality.
)

(fn ConstructionScript
  (|CallParentFunction))

(fn Activate
  (|CallParentFunction)
  (CallFunction|LeverActivate)
  (CallFunction|OpenStone))

(fn CheckCondition
  (return true))