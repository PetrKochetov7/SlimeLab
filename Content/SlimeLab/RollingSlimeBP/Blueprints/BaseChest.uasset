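; BaseChest is a locked chest that opens when activated if the player's MainCharacter inventory contains its MyKey.
; Activate runs CheckCondition, then either calls OpenTop or TextNeed, which briefly shows a text prompt when the key is missing.
; Overlapping the Box also triggers TextNeed.
; OpenTop fires once, animating the lid with MoveComponentTo while spawning a BP_PickUp_Crystal at the chest after a short delay.
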(event OnComponentBeginOverlap(Box)
  (params (OverlappedComponent :type Primitive%20Component%20Object%20Reference) (OtherActor :type Actor%20Object%20Reference) (OtherComp :type Primitive%20Component%20Object%20Reference) (OtherBodyIndex :type Integer) (bFromSweep :type Boolean) (SweepResult :type Hit%20Result%20Structure%20%28by%20ref%29))
  (CallFunction|TextNeed))

(event Custom|OpenTop
  (Utilities|FlowControl|DoOnce false
    (:Completed
      (Utilities|FlowControl|Sequence
        (:then_0
          (Utilities|FlowControl|Delay 0.7)
          (Game|SpawnActorfromClass "/Game/SlimeLab/PickUpAndCrystal/BP_PickUp_Crystal.BP_PickUp_Crystal_C" (Math|Transform|MakeTransform (Transformation|GetActorLocation) (Transformation|GetActorRotation) (+ (Transformation|GetActorScale3D) 1.0)) "AdjustIfPossibleButAlwaysSpawn" (Variables|Default|GetCrystal) 0))
        (:then_1
          (Components|MoveComponentTo (Variables|Default|GetStaticMesh1) "1.000000,19.770000,37.000000" "0, 0,90.000000" false false 1.0 false))))))

(event Custom|TextNeed
  (bind _asmain_character (Utilities|Casting|CastToMainCharacter (Game|Player|GetPlayerPawn 0)))
  (if (not (Utilities|Array|ContainsItem (Variables|/Game/SlimeLab/RollingSlimeBP/Blueprints/MainCharacter.MainCharacter_C|GetInventory _asmain_character) (Variables|Default|GetMyKey)))
    (Rendering|SetVisibility (Variables|Default|GetTextRender) true false)
    (Utilities|FlowControl|Delay 3.0)
    (Rendering|SetVisibility (Variables|Default|GetTextRender) false false)))

(event EventBeginPlay
  (|CallParentFunction)
  (Rendering|SetVisibility (Variables|Default|GetTextRender) false false))

(event Collision|EventActorBeginOverlap
  (params (OtherActor :type Actor%20Object%20Reference))
  (|CallParentFunction OtherActor) ; This node is disabled and will not be called.\nDrag off pins to build functionality.
)

(event EventTick
  (params (DeltaSeconds :type Float%20%28single-precision%29))
  (|CallParentFunction DeltaSeconds) ; This node is disabled and will not be called.\nDrag off pins to build functionality.
)

(fn ConstructionScript
  (|CallParentFunction))

(fn CheckCondition
  (bind _asmain_character (Utilities|Casting|CastToMainCharacter (Game|Player|GetPlayerPawn 0))
    (:then
      (return (Utilities|Array|ContainsItem (Variables|/Game/SlimeLab/RollingSlimeBP/Blueprints/MainCharacter.MainCharacter_C|GetInventory _asmain_character) (Variables|Default|GetMyKey))))
    (:CastFailed
      (return false))))

(fn Activate
  (|CallParentFunction)
  (if (CallFunction|CheckCondition)
    (CallFunction|OpenTop)
    (else
      (CallFunction|TextNeed))))