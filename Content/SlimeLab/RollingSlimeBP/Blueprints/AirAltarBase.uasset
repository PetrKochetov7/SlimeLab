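; Air altar actor that switches the main character to a new team form, presumably air, when they enter its box.
; The box overlap shows the altar text and calls ChangeForm, which sets Team, hides the text and, after a delay, spawns a temporary Niagara wind burst while restyling the ball material and light.
; Activate and CheckCondition only defer to the parent class.
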(event OnComponentBeginOverlap(Box)
  (params (OverlappedComponent :type Primitive%20Component%20Object%20Reference) (OtherActor :type Actor%20Object%20Reference) (OtherComp :type Primitive%20Component%20Object%20Reference) (OtherBodyIndex :type Integer) (bFromSweep :type Boolean) (SweepResult :type Hit%20Result%20Structure%20%28by%20ref%29))
  ;[1 1 1] Interaction with Main Character
  (Rendering|SetVisibility (Variables|Default|GetTextRender) true false)
  (bind _asmain_character (Utilities|Casting|CastToMainCharacter OtherActor))
  (CallFunction|ChangeForm _asmain_character))

(event OnComponentEndOverlap(Box)
  (params (OverlappedComponent :type Primitive%20Component%20Object%20Reference) (OtherActor :type Actor%20Object%20Reference) (OtherComp :type Primitive%20Component%20Object%20Reference) (OtherBodyIndex :type Integer))
  ;[1 1 1] Interaction with Main Character
  (Rendering|SetVisibility (Variables|Default|GetTextRender) false false))

(event Custom|ChangeForm
  (params (Player :type Main%20Character%20Object%20Reference))
  (bind _pointlight (Variables|/Game/SlimeLab/RollingSlimeBP/Blueprints/MainCharacter.MainCharacter_C|GetPointLight Player))
  ;[1 1 1] Change form(team)
  (Variables|/Game/SlimeLab/RollingSlimeBP/Blueprints/MainCharacter.MainCharacter_C|SetTeam Player "NewEnumerator2")
  ;[1 1 1] Text on altar
  (Rendering|SetVisibility (Variables|Default|GetTextRender) false false)
  ;[1 1 1] Animation on altar
  (Utilities|FlowControl|Delay 1.0)
  (bind _returnvalue (Niagara|SpawnSystematLocation "/Game/SlimeLab/DownloadContentent/sA_PickupSet_1/Fx/NiagaraSystems/NS_Pickup_Wind.NS_Pickup_Wind" (Transformation|GetActorLocation Player) "0, 0, 0" "5.000000,5.000000,5.000000"))
  (Rendering|Material|SetMaterial (Variables|/Game/SlimeLab/RollingSlimeBP/Blueprints/MainCharacter.MainCharacter_C|GetBall Player) 0 "/Game/SlimeLab/DownloadContentent/GlassPack/Materials/01_Clean/_Examples/M_Glass_Acrylic.M_Glass_Acrylic")
  (Rendering|Components|Light|SetLightColor _pointlight "(R=0.000000,G=0.984000,B=0.698952,A=1.000000)" true)
  (Rendering|Components|Light|SetIntensity _pointlight 3.5e+04)
  (Utilities|FlowControl|Delay 1.0)
  (Components|DestroyComponent _returnvalue))

(event EventBeginPlay
  (|CallParentFunction))

(event Collision|EventActorBeginOverlap
  (params (OtherActor :type Actor%20Object%20Reference))
  (|CallParentFunction OtherActor))

(event EventTick
  (params (DeltaSeconds :type Float%20%28single-precision%29))
  (|CallParentFunction DeltaSeconds) ; This node is disabled and will not be called.\nDrag off pins to build functionality.
)

(fn ConstructionScript
  (|CallParentFunction))

(fn Activate
  (|CallParentFunction))

(fn CheckCondition
  (return (|CallParentFunction)))